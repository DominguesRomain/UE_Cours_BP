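; BP_Interrupter is a proximity light switch that controls the PointLight of a referenced Lumos object through a Box trigger.
; Beginning an overlap turns the light on at high intensity, and ending it turns the light off after a fixed Delay, with debug prints on entry.
; Both events cast player 0's character to BP_ThirdPersonCharacter rather than checking the overlapping actor, so other actors can also trigger it.
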(event OnComponentBeginOverlap(Box)
  (params (OverlappedComponent :type Primitive%20Component%20Object%20Reference) (OtherActor :type Actor%20Object%20Reference) (OtherComp :type Primitive%20Component%20Object%20Reference) (OtherBodyIndex :type Integer) (bFromSweep :type Boolean) (SweepResult :type Hit%20Result%20Structure%20%28by%20ref%29))
  (Utilities|Casting|CastToBP_ThirdPersonCharacter (Game|GetPlayerCharacter 0)
    (:then
      (Development|PrintString "oui")
      (Rendering|Components|Light|SetIntensity (Variables|/Game/Blueprint/BP_Light.BP_Light_C|GetPointLight (Variables|Default|Getlumos)) 1e+03))
    (:CastFailed
      (Development|PrintString "non"))))

(event OnComponentEndOverlap(Box)
  (params (OverlappedComponent :type Primitive%20Component%20Object%20Reference) (OtherActor :type Actor%20Object%20Reference) (OtherComp :type Primitive%20Component%20Object%20Reference) (OtherBodyIndex :type Integer))
  (Utilities|Casting|CastToBP_ThirdPersonCharacter (Game|GetPlayerCharacter 0))
  (Utilities|FlowControl|Delay 5.0)
  (Rendering|Components|Light|SetIntensity (Variables|/Game/Blueprint/BP_Light.BP_Light_C|GetPointLight (Variables|Default|Getlumos)) 0.0))

(fn ConstructionScript)